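; BP_Wall_Obstacle is a wall obstacle that triggers the outro screen when a snake character overlaps it.
; On overlap it gets the snake's controller and reads player data from the SnakeGameInstance.
; In co-op mode it passes the other player's ID and score to ShowOutro on the colliding snake's controller.
; Otherwise it passes player 1's ID and score.
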(event Collision|EventActorBeginOverlap
  (params (OtherActor :type Actor%20Object%20Reference))
  ;[0.15 0.9478 0.15 0.5] Begin Overlap
  (bind _asbp_snake_character_new (Utilities|Casting|CastToBP_SnakeCharacter_New OtherActor))
  (bind _asbp_snake_controller (Utilities|Casting|CastToBP_SnakeController (Pawn|GetController _asbp_snake_character_new)))
  (Variables|Default|SetAs%20BP%20Snake%20Controller _asbp_snake_controller)
  (bind _assnake_game_instance (Utilities|Casting|CastToSnakeGameInstance (Game|GetGameInstance)))
  (Variables|Default|SetAs%20Snake%20Game%20Instance _assnake_game_instance)
  (if (Class|SnakeGameInstance|IsCoopMode _assnake_game_instance)
    (if (== (Class|GameplayStatics|GetPlayerControllerID (Game|GetPlayerController (Variables|/Script/Engine.Controller|GetPlayerState (Pawn|GetController _asbp_snake_character_new)))) 0)
      (bind _returnvalue (Class|SnakeGameInstance|GetSnakePlayerData (Variables|Default|GetAs%20Snake%20Game%20Instance) 1))
      (Default|ShowOutro (Variables|Default|GetAs%20BP%20Snake%20Controller) 2 (.score _returnvalue))
      (else
        (bind _returnvalue_2 (Class|SnakeGameInstance|GetSnakePlayerData (Variables|Default|GetAs%20Snake%20Game%20Instance)))
        (Default|ShowOutro (Variables|Default|GetAs%20BP%20Snake%20Controller) 1 (.score _returnvalue_2))))
    (else
      (bind _returnvalue_3 (Class|SnakeGameInstance|GetSnakePlayerData (Variables|Default|GetAs%20Snake%20Game%20Instance)))
      (Default|ShowOutro (Variables|Default|GetAs%20BP%20Snake%20Controller) 1 (.score _returnvalue_3)))))

(fn ConstructionScript)
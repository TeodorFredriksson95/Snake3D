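; BP_Wall_Obstacle_Tower is a wall obstacle that triggers the outro when a snake character overlaps it.
; On overlap it casts the actor to SnakeCharacter and its controller to BP_SnakeController, ignoring anything else.
; It reads the player controller ID and calls ShowOutro on that controller with the opposite index, presumably naming the other player as winner.
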(event Collision|EventActorBeginOverlap
  (params (OtherActor :type Actor%20Object%20Reference))
  (bind _assnake_character (Utilities|Casting|CastToSnakeCharacter OtherActor))
  (bind _asbp_snake_controller (Utilities|Casting|CastToBP_SnakeController (Pawn|GetController _assnake_character)))
  (Variables|Default|SetAs%20BP%20Snake%20Controller _asbp_snake_controller)
  (if (== (Class|GameplayStatics|GetPlayerControllerID (Game|GetPlayerController (Variables|/Script/Engine.Controller|GetPlayerState (Pawn|GetController _assnake_character)))) 0)
    (Default|ShowOutro (Variables|Default|GetAs%20BP%20Snake%20Controller) 1)
    (else
      (Default|ShowOutro (Variables|Default|GetAs%20BP%20Snake%20Controller)))))

(fn ConstructionScript)
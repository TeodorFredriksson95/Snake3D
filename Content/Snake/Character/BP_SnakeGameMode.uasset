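; BP_SnakeGameMode is the Snake game mode, which handles player setup and level progression when a target score is reached.
; On BeginPlay it sets the game state to Game, binds to the first player's BP_SnakeState score event, and creates a second local player.
; PostLogin binds the same event for each joining player's BP_SnakeState.
; HandleScoreReached switches on the current level to open the corresponding map by name.
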(event Custom|HandleScoreReached
  (params (CurrentLevel :type ESnakeGameLevel%20Enum :default "FirstLevel"))
  (switch Utilities|FlowControl|Switch|SwitchonESnakeGameLevel CurrentLevel
    (:SecondLevel
      (Game|OpenLevel(byName) "Lvl_ThirdPerson"))
    (:ThirdLevel
      (Game|OpenLevel(byName) "Lvl_SnakeLevel_01"))))

(event EventBeginPlay
  (bind _asbp_snake_game_mode (Utilities|Casting|CastToBP_SnakeGameMode (Game|GetGameMode)))
  (Class|SnakeGameMode|SetGameState _asbp_snake_game_mode "Game")
  (bind _asbp_snake_state (Utilities|Casting|CastToBP_SnakeState (Game|GetPlayerState 0)))
  (EventDispatchers|BindEventtoOnReachedTargetScore _asbp_snake_state (delegate Custom|HandleScoreReached))
  (Class|GameplayStatics|CreatePlayer 1))

(event EventPostLogin
  (params (NewPlayer :type Player%20Controller%20Object%20Reference))
  (bind _asbp_snake_state (Utilities|Casting|CastToBP_SnakeState (Variables|/Script/Engine.Controller|GetPlayerState NewPlayer)))
  (EventDispatchers|BindEventtoOnReachedTargetScore _asbp_snake_state (delegate Custom|HandleScoreReached)))

(fn ConstructionScript)